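; Balloon actor that can be picked up, dropped off and popped.
; PickUp enables physics simulation on the balloon mesh and attaches the root to the given actor, keeping world transforms.
; DropOff detaches it, keeps physics on and launches the mesh with a fixed forward-and-up world impulse.
; Popped only plays a pop sound at the mesh location, without destroying or hiding the balloon.
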(event Custom|Popped
  (Audio|PlaySoundatLocation "/Game/Assets/audio/a_balloonPop_Cue.a_balloonPop_Cue" (Transformation|GetWorldLocation (Variables|Default|Getballoon_mesh))))

(event Collision|EventActorBeginOverlap
  (params (OtherActor :type Actor%20Object%20Reference)))

(event EventDropOff
  (Physics|SetSimulatePhysics (Variables|Default|Getballoon_mesh) true)
  (Transformation|DetachFromActor "KeepWorld" "KeepWorld" "KeepWorld")
  (Physics|AddImpulse (Variables|Default|Getballoon_mesh) "500.000000,0.000000,500.000000" "None" false))

(event EventTick
  (params (DeltaSeconds :type Float%20%28single-precision%29)))

(event EventPickUp
  (params (ActorToAttachTo :type Scene%20Component%20Object%20Reference))
  (Physics|SetSimulatePhysics (Variables|Default|Getballoon_mesh) true)
  (Transformation|AttachComponentToComponent (Variables|Transformation|GetRootComponent) ActorToAttachTo "None" "KeepWorld" "KeepWorld" "KeepWorld" true))

(fn ConstructionScript)